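; BP_InventorySlot is a VR inventory slot actor that detects inventory items inside its sphere.
; Sphere overlap events store the latest overlapping InventoryItemClass actor and clear the reference when that same item leaves.
; The Put event calls TryGrab on the stored item's GrabComponent with MotionController, without checking that an item is present.
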(event `self.Sphere.OnComponentBeginOverlap`
  (params (OverlappedComponent :type "PrimitiveComponent Object Reference") (OtherActor :type "Actor Object Reference") (OtherComp :type "PrimitiveComponent Object Reference") (OtherBodyIndex :type Integer) (bFromSweep :type Boolean) (SweepResult :type "HitResult Structure (by ref)"))
  (bind _asinventory_item_class (cast `/Game/New_BP/Class/InventoryItemClass` OtherActor))
  (set `self.As Inventory Item Class` _asinventory_item_class))

(event `self.Sphere.OnComponentEndOverlap`
  (params (OverlappedComponent :type "PrimitiveComponent Object Reference") (OtherActor :type "Actor Object Reference") (OtherComp :type "PrimitiveComponent Object Reference") (OtherBodyIndex :type Integer))
  (bind _asinventory_item_class (cast `/Game/New_BP/Class/InventoryItemClass` OtherActor))
  (if (== _asinventory_item_class (`self.As Inventory Item Class`))
    (set `self.As Inventory Item Class` null)))

(event `Put`
  (`/Game/VRTemplate/Blueprints/GrabComponent.TryGrab` (`/Game/New_BP/Class/BP_Interaction_Class.GrabComponent` (`self.As Inventory Item Class`)) (`self.MotionController`)))

(fn `UserConstructionScript`)