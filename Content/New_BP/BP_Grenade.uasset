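; BP_Grenade is a grenade actor with a five-second fuse that begins when TriggerReleased is called.
; That event starts a looping one-second timer bound to the 5Sec event, where a DoN node counts the ticks.
; Each tick prints the remaining count, and the fifth prints a boom message and destroys the actor.
; The blast is only debug text, with no damage or effects.
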(event `/Game/VRTemplate/Blueprints/VRInteractionBPI.TriggerReleased`
  (`KismetSystemLibrary.K2_SetTimerDelegate` (delegate `5Sec`) 1.0 true))

(event `5Sec`
  (bind _counter (`/Engine/EditorBlueprintResources/StandardMacros.Do N` 5)
    (:`Exit`
      (if (== _counter 5)
        (`KismetSystemLibrary.PrintString` "BOOOM")
        (`self.K2_DestroyActor`)
        (else
          (`KismetSystemLibrary.PrintString` (`KismetStringLibrary.Conv_IntToString` (- 5 _counter))))))))

(fn `UserConstructionScript`
  (`parent.UserConstructionScript`))